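; BP_DamageReceiver is a component that tracks its owner's health and applies incoming damage.
; On BeginPlay, a BP_Character owner takes its saved HP from BP_GameInstance, while any other owner starts at max health.
; An accepted hit opens a timed invulnerability window, subtracts the damage and broadcasts the health change.
; At zero or below, health is set to zero and OnDead fires before that broadcast.
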(event Custom|OnDamageReceived
  (params (Damage :type Float%20%28double-precision%29))
  (if (Variables|Default|Getvulnerable)
    (Variables|Default|Setvulnerable false)
    (Utilities|Time|SetTimerbyEvent (delegate Custom|ReturnToVulnerable) (Variables|Default|GetInvulnerableTime))
    (Variables|Default|SetCurrentHealthPower (- (Variables|Default|GetCurrentHealthPower) Damage))
    (if (<= (Variables|Default|GetCurrentHealthPower) 0.0)
      (Variables|Default|SetCurrentHealthPower 0.0)
      (Default|CallOnDead)
      (Default|CallOnHealthPowerChanged (Variables|Default|GetMaxHealthPower) (Variables|Default|GetCurrentHealthPower))
      (else
        (Default|CallOnHealthPowerChanged (Variables|Default|GetMaxHealthPower) (Variables|Default|GetCurrentHealthPower))))))

(event Custom|ReturnToVulnerable
  (Variables|Default|Setvulnerable true))

(event EventBeginPlay
  (Utilities|Casting|CastToBP_Character (Components|GetOwner)
    (:then
      (bind _asbp_game_instance (Utilities|Casting|CastToBP_GameInstance (Game|GetGameInstance)))
      (Variables|Default|SetCurrentHealthPower (Variables|/Game/Blueprint/Character/BP_GameInstance.BP_GameInstance_C|GetPlayerCurrentHP _asbp_game_instance)))
    (:CastFailed
      (Variables|Default|SetCurrentHealthPower (Variables|Default|GetMaxHealthPower)))))

(event EventTick
  (params (DeltaSeconds :type Float%20%28single-precision%29)))