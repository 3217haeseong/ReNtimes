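; Skill component that loads JumpSlash, CutDown and DamageBuff from the SkillData table and tracks whether each can be used.
; UseSkill looks up the named row, plays its section of AM_Skill on the player character and returns its value.
; Buff-type skills also adjust weapon damage or character AttackDamage by the chosen stat, with a timer calling Rollback partway through the cooldown.
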(event EventBeginPlay
  (bind _skilldata (CallFunction|GetDatabyName "JumpSlash"))
  (Utilities|Array|AddUnique (Variables|Default|GetSkill) _skilldata)
  (bind _skilldata_2 (CallFunction|GetDatabyName "CutDown"))
  (Utilities|Array|AddUnique (Variables|Default|GetSkill) _skilldata_2)
  (bind _skilldata_3 (CallFunction|GetDatabyName "DamageBuff"))
  (Utilities|Array|AddUnique (Variables|Default|GetSkill) _skilldata_3))

(fn UseSkill
  (params (SkillName :type Name))
  (bind _skilldata (CallFunction|GetDatabyName SkillName))
  (if (Utilities|Enum|Equal(Enum) (.Type (Utilities|Struct|BreakSkillStructure _skilldata)) "NewEnumerator1")
    (CallFunction|Buff (.Value (Utilities|Struct|BreakSkillStructure _skilldata)) (.ApplyStat (Utilities|Struct|BreakSkillStructure _skilldata)))
    (Utilities|Time|SetTimerbyFunctionName 0 "Rollback" (* (.CoolDown (Utilities|Struct|BreakSkillStructure _skilldata)) 0.66)))
  (bind _asbp_character (Utilities|Casting|CastToBP_Character (Game|GetPlayerCharacter 0)))
  (Animation|PlayAnimMontage _asbp_character "/Game/Blueprint/Skill/Animation/AM_Skill.AM_Skill" 1.0 (.Section (Utilities|Struct|BreakSkillStructure _skilldata)))
  (return (.Value (Utilities|Struct|BreakSkillStructure _skilldata))))

(fn CanUse
  (params (SkillIndex :type Integer))
  (return (.CanUse (Utilities|Struct|BreakSkillStructure (Utilities|Array|Get(acopy) (Variables|Default|GetSkill) SkillIndex)))))

(fn GetDatabyName
  (params (SkillName :type Name))
  (bind _skilldata (Variables|Default|GetSkillData))
  (Utilities|IsValid _skilldata
    (:Is%20Valid
      (bind _returnvalue (Utilities|GetDataTableRow _skilldata SkillName)
        (:then
          (return _returnvalue))))))

(fn SetSkillCanUse
  (params (SkillIndex :type Integer) (CanUse :type Boolean))
  (bind _skill (Variables|Default|GetSkill))
  (bind _output (Utilities|Array|Get(acopy) _skill SkillIndex))
  (Utilities|Array|SetArrayElem (Variables|Default|GetSkill) SkillIndex (Utilities|Struct|MakeSkillStructure (.cooldown _output) (.value _output) (.section _output) (.effect _output) (.type _output) (.applystat _output) CanUse)))

(fn Buff
  (params (Value :type Float%20%28double-precision%29) (ApplyStat :type Name))
  (Variables|Default|SetApplyStat ApplyStat)
  (bind _asbp_character (Utilities|Casting|CastToBP_Character (Game|Player|GetPlayerPawn 0)))
  (switch name ApplyStat
    (:AttackDamage
      (Variables|/Game/Blueprint/Character/Weapon/BP_Weapon.BP_Weapon_C|SetBase%20Damage (Variables|/Game/Blueprint/Character/BP_Character.BP_Character_C|GetWeapon _asbp_character) (+ (Variables|/Game/Blueprint/Character/Weapon/BP_Weapon.BP_Weapon_C|GetBase%20Damage (Variables|/Game/Blueprint/Character/BP_Character.BP_Character_C|GetWeapon _asbp_character)) Value)))
    (:CurrentAttackSpeed
      (Variables|/Game/Blueprint/Character/BP_Character.BP_Character_C|SetAttackDamage _asbp_character (+ Value (Variables|/Game/Blueprint/Character/BP_Character.BP_Character_C|GetCurrentAttackSpeed _asbp_character)))))
  (return))

(fn RollBack
  (bind _asbp_character (Utilities|Casting|CastToBP_Character (Game|Player|GetPlayerPawn 0)))
  (switch name (Variables|Default|GetApplyStat)
    (:AttackDamage
      (Variables|/Game/Blueprint/Character/Weapon/BP_Weapon.BP_Weapon_C|SetBase%20Damage (Variables|/Game/Blueprint/Character/BP_Character.BP_Character_C|GetWeapon _asbp_character) (- (Variables|/Game/Blueprint/Character/Weapon/BP_Weapon.BP_Weapon_C|GetBase%20Damage (Variables|/Game/Blueprint/Character/BP_Character.BP_Character_C|GetWeapon _asbp_character)) (Variables|Default|GetValue))))
    (:CurrentAttackSpeed
      (Variables|/Game/Blueprint/Character/BP_Character.BP_Character_C|SetAttackDamage _asbp_character (- (Variables|/Game/Blueprint/Character/BP_Character.BP_Character_C|GetCurrentAttackSpeed _asbp_character) (Variables|Default|GetValue)))))
  (return))