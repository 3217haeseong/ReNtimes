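; AI controller for the bear monster, which starts its behavior tree when it possesses a pawn.
; On possess it initializes the BB_MonsterBear blackboard, seeding the skill wait time and storing the pawn's current location as its origin.
; It then runs BT_MonsterBear, leaving all further decision-making to that tree.
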(event EventPossess
  (params (PossessedPawn :type Pawn%20Object%20Reference))
  (Utilities|FlowControl|Sequence
    (:then_0
      (Class|AIController|UseBlackboard "/Game/Blueprint/Monster/AI/BB_MonsterBear.BB_MonsterBear")
      (AI|Components|Blackboard|SetValueasFloat (Variables|Default|GetBlackboard) (Variables|Default|GetSkillWaitTimeKey) (Variables|Default|GetSkillWaitTime))
      (AI|Components|Blackboard|SetValueasVector (Variables|Default|GetBlackboard) (Variables|Default|GetSetOriginLocationKey) (Transformation|GetActorLocation PossessedPawn)))
    (:then_1
      (AI|RunBehaviorTree "/Game/Blueprint/Monster/AI/BT_MonsterBear.BT_MonsterBear"))))

(fn ConstructionScript)