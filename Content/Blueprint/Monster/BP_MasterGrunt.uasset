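; Master Grunt monster character that carries a spawned weapon on its hand socket, shows an HP bar and tags the MainDoor with a gimmick-open event after dying.
; A state machine mirrors each state to the AI blackboard and sets walk speed from monster data, with Dead as terminal.
; Pawn sensing starts chases on player characters, while Tick returns it to Ready from Chase or Attack based on sight radius or player state.
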(event OnSeePawn(PawnSensing)
  (params (Pawn :type Pawn%20Object%20Reference))
  (switch Utilities|FlowControl|Switch|SwitchonEGruntState (Variables|Default|GetBP_State)
    (:NewEnumerator1
      _)
    (:NewEnumerator2
      _))
  (bind _asbp_character (Utilities|Casting|CastToBP_Character Pawn))
  (if (Utilities|Enum|NotEqual(Enum) (Variables|/Game/Blueprint/Character/BP_Character.BP_Character_C|GetCharacterState _asbp_character) "NewEnumerator2")
    (AI|Components|Blackboard|SetValueasObject (Variables|/Script/AIModule.AIController|GetBlackboard (AI|GetAIController self)) (Variables|Default|GetTargetPlayerKey) Pawn)
    (CallFunction|SetState "NewEnumerator2")))

(event Custom|SetState
  (params (NewState :type EGruntState%20Enum :default "NewEnumerator0"))
  (bind _monsterdata (Variables|Default|GetMonsterData))
  (bind _currentleveldata (Default|GetCurrentLevelData _monsterdata))
  (if (Utilities|Enum|NotEqual(Enum) (Variables|Default|GetBP_State) NewState)
    (if (Utilities|Enum|NotEqual(Enum) (Variables|Default|GetBP_State) "NewEnumerator5")
      (AI|Components|Blackboard|SetValueasEnum (AI|GetBlackboard (AI|GetAIController self)) (Variables|Default|GetStateKey) NewState)
      (bind _output_get (Variables|Default|SetBP_State NewState))
      (switch Utilities|FlowControl|Switch|SwitchonEGruntState _output_get
        (:NewEnumerator0
          (Variables|/Script/Engine.CharacterMovementComponent|SetMaxWalkSpeed (Variables|Character|GetCharacterMovement) 0.0 :!label _label))
        (:NewEnumerator1
          (Variables|/Script/Engine.CharacterMovementComponent|SetMaxWalkSpeed (Variables|Character|GetCharacterMovement) (.walkspeed _currentleveldata))
          (AI|Components|Blackboard|SetValueasObject (AI|GetBlackboard (AI|GetAIController self)) (Variables|Default|GetTargetPlayerKey) 0))
        (:NewEnumerator2
          (Variables|/Script/Engine.CharacterMovementComponent|SetMaxWalkSpeed (Variables|Character|GetCharacterMovement) (.chasespeed _currentleveldata)))
        (:NewEnumerator3
          (goto _label))
        (:NewEnumerator4
          (goto _label))
        (:NewEnumerator5
          (goto _label))))))

(event Custom|OnGruntDead
  (CallFunction|SetState "NewEnumerator5")
  (Utilities|FlowControl|Delay 2.0)
  (Actor|DestroyActor)
  (Ability|GameplayEffect|AddLooseGameplayTags (Variables|Default|GetTarget) (GameplayTags|MakeGameplayTagContainerfromTag "(TagName=\"Event.Gimmick.Open\")")))

(event Custom|OnHpChanged
  (params (MaxHealthPower :type Float%20%28double-precision%29) (currentHealthPower :type Float%20%28double-precision%29))
  (Default|SetHPPercent (Variables|Default|GetHPBarObject) (/ currentHealthPower MaxHealthPower)))

(event Custom|TurnToTarget
  (params (Target :type Actor%20Object%20Reference))
  (Transformation|SetActorRotation (Math|Rotator|MakeRotator 0.0 0.0 (.yaw (Math|Rotator|MakeRotfromX (- (Transformation|GetActorLocation Target) (Transformation|GetActorLocation)))))))

(event Custom|OnReady
  (CallFunction|SetState "NewEnumerator1"))

(event EventBeginPlay
  (bind _returnvalue (Game|SpawnActorfromClass "/Game/Blueprint/Monster/BP_GruntWeapon.BP_GruntWeapon_C" (Math|Transform|MakeTransform "0.000000,0.000000,0.000000" "0.000000,0.000000,0.000000") "Undefined" "MultiplyWithRoot" 0 0))
  (Transformation|AttachComponentToComponent _returnvalue (Variables|Character|GetMesh) "b_MF_Weapon_R" "SnapToTarget" "SnapToTarget" "SnapToTarget" true)
  (Transformation|SetActorRelativeTransform _returnvalue (Math|Transform|MakeTransform "12.000000,-2.600000,0.000000" "0.000000,-90.000000,90.000000" "1.000000,1.000000,1.000000") false false)
  (bind _returnvalue_2 (Actor|GetActorOfClass "/Game/Blueprint/Actor/MainDoor.MainDoor_C"))
  (Variables|Default|SetTarget _returnvalue_2)
  (EventDispatchers|BindEventtoOnDead (Variables|Default|GetDamageReceiver) (delegate Custom|OnGruntDead))
  (bind _aswbp_monster_hp (Utilities|Casting|CastToWBP_MonsterHp (UserInterface|GetUserWidgetObject (Variables|Default|GetHPBar))))
  (Variables|Default|SetHPBarObject _aswbp_monster_hp)
  (EventDispatchers|BindEventtoOnHealthPowerChanged (Variables|Default|GetDamageReceiver) (delegate Custom|OnHpChanged))
  (Variables|/Script/Engine.CharacterMovementComponent|SetMaxWalkSpeed (Variables|Character|GetCharacterMovement) (.walkspeed (Default|GetCurrentLevelData (Variables|Default|GetMonsterData)))))

(event EventTick
  (params (DeltaSeconds :type Float%20%28single-precision%29))
  (switch Utilities|FlowControl|Switch|SwitchonEGruntState (Variables|Default|GetBP_State)
    (:NewEnumerator2
      (CallFunction|OnChase))
    (:NewEnumerator3
      (CallFunction|OnAttack))))

(fn ConstructionScript)

(fn OnChase
  (bind _asactor (Utilities|Casting|CastToActor (AI|Components|Blackboard|GetValueasObject (AI|GetBlackboard (AI|GetAIController self)) (Variables|Default|GetTargetPlayerKey))))
  (if (> (Transformation|GetDistanceTo _asactor 0) (Variables|/Script/AIModule.PawnSensingComponent|GetSightRadius (Variables|Default|GetPawnSensing)))
    (CallFunction|SetState "NewEnumerator1")))

(fn OnAttack
  (bind _asbp_character (Utilities|Casting|CastToBP_Character (AI|Components|Blackboard|GetValueasObject (AI|GetBlackboard (AI|GetAIController self)) (Variables|Default|GetTargetPlayerKey))))
  (if (Utilities|Enum|NotEqual(Enum) (Variables|/Game/Blueprint/Character/BP_Character.BP_Character_C|GetCharacterState _asbp_character) "NewEnumerator2")
    (CallFunction|SetState "NewEnumerator1")))