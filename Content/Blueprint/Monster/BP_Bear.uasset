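; Bear monster character that spots, chases and attacks the player, with a widget health bar.
; A state machine mirrors its state to the Blackboard and sets movement speed from MonsterData or zero.
; PawnSensing starts chases, while Tick returns it to Ready when the target leaves sight radius during Chase or enters an excluded state during Attack.
; DamageReceiver drives the health bar and death, which disables collisions and delays destruction.
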(event OnSeePawn(PawnSensing)
  (params (Pawn :type Pawn%20Object%20Reference))
  (switch Utilities|FlowControl|Switch|SwitchonEBearState (Variables|Default|GetState_BP)
    (:NewEnumerator0
      _)
    (:NewEnumerator1
      _))
  (bind _asbp_character (Utilities|Casting|CastToBP_Character Pawn))
  (if (Utilities|Enum|NotEqual(Enum) (Variables|/Game/Blueprint/Character/BP_Character.BP_Character_C|GetCharacterState _asbp_character) "NewEnumerator2")
    (AI|Components|Blackboard|SetValueasObject (Variables|/Script/AIModule.AIController|GetBlackboard (AI|GetAIController self)) (Variables|Default|GetTargetPlayerKey) Pawn)
    (CallFunction|SetState "NewEnumerator1")))

(event Custom|SetState
  (params (NewState :type EBearState%20Enum :default "NewEnumerator0"))
  (bind _monsterdata (Variables|Default|GetMonsterData))
  (bind _currentleveldata (Default|GetCurrentLevelData _monsterdata))
  (if (Utilities|Enum|NotEqual(Enum) (Variables|Default|GetState_BP) "NewEnumerator4")
    (if (Utilities|Enum|NotEqual(Enum) NewState (Variables|Default|GetState_BP))
      (AI|Components|Blackboard|SetValueasEnum (AI|GetBlackboard (AI|GetAIController self)) (Variables|Default|GetStateKey) NewState)
      (bind _output_get (Variables|Default|SetState_BP NewState))
      (switch Utilities|FlowControl|Switch|SwitchonEBearState _output_get
        (:NewEnumerator0
          (Variables|/Script/Engine.CharacterMovementComponent|SetMaxWalkSpeed (Variables|Character|GetCharacterMovement) (.walkspeed _currentleveldata))
          (AI|Components|Blackboard|SetValueasObject (AI|GetBlackboard (AI|GetAIController self)) (Variables|Default|GetTargetPlayerKey) 0))
        (:NewEnumerator1
          (Variables|/Script/Engine.CharacterMovementComponent|SetMaxWalkSpeed (Variables|Character|GetCharacterMovement) (.chasespeed _currentleveldata)))
        (:NewEnumerator2
          (Variables|/Script/Engine.CharacterMovementComponent|SetMaxWalkSpeed (Variables|Character|GetCharacterMovement) 0.0 :!label _label))
        (:NewEnumerator4
          (goto _label))
        (:NewEnumerator5
          (goto _label))))))

(event Custom|TurnToTarget
  (params (Target :type Actor%20Object%20Reference))
  (Transformation|SetActorRotation (Math|Rotator|MakeRotator 0.0 0.0 (.yaw (Math|Rotator|MakeRotfromX (- (Transformation|GetActorLocation Target) (Transformation|GetActorLocation)))))))

(event Custom|OnReady
  (CallFunction|SetState "NewEnumerator0"))

(event Custom|OnMonsterDead
  (Collision|SetCollisionEnabled (Variables|Collision|GetCapsuleComponent) "NoCollision")
  (Collision|SetCollisionEnabled (Variables|Default|GetRightCollision) "NoCollision")
  (Collision|SetCollisionEnabled (Variables|Default|GetLeftCollision) "NoCollision")
  (CallFunction|SetState "NewEnumerator4")
  (Utilities|FlowControl|Delay 2.0)
  (Actor|DestroyActor))

(event Custom|OnHPChanged
  (params (MaxHealthPower :type Float%20%28double-precision%29) (currentHealthPower :type Float%20%28double-precision%29))
  (Default|SetHPPercent (Variables|Default|GetHPBarObject) (/ currentHealthPower MaxHealthPower)))

(event EventBeginPlay
  (EventDispatchers|BindEventtoOnDead (Variables|Default|GetDamageReceiver) (delegate Custom|OnMonsterDead))
  (bind _aswbp_monster_hp (Utilities|Casting|CastToWBP_MonsterHp (UserInterface|GetUserWidgetObject (Variables|Default|GetHPBar))))
  (Variables|Default|SetHPBarObject _aswbp_monster_hp)
  (EventDispatchers|BindEventtoOnHealthPowerChanged (Variables|Default|GetDamageReceiver) (delegate Custom|OnHPChanged))
  (Variables|/Script/Engine.CharacterMovementComponent|SetMaxWalkSpeed (Variables|Character|GetCharacterMovement) (.walkspeed (Default|GetCurrentLevelData (Variables|Default|GetMonsterData)))))

(event Collision|EventActorBeginOverlap
  (params (OtherActor :type Actor%20Object%20Reference))
  (Variables|/Script/Engine.CharacterMovementComponent|SetMaxWalkSpeed (Variables|Character|GetCharacterMovement) (.walkspeed (Default|GetCurrentLevelData (Variables|Default|GetMonsterData)))))

(event EventTick
  (params (DeltaSeconds :type Float%20%28single-precision%29))
  (switch Utilities|FlowControl|Switch|SwitchonEBearState (Variables|Default|GetState_BP)
    (:NewEnumerator1
      (CallFunction|OnChase))
    (:NewEnumerator2
      (CallFunction|OnAttack))))

(event Game|Damage|EventAnyDamage
  (params (Damage :type Float%20%28single-precision%29) (DamageType :type Damage%20Type%20Object%20Reference) (InstigatedBy :type Controller%20Object%20Reference) (DamageCauser :type Actor%20Object%20Reference))
  (Default|OnDamageReceived (Variables|Default|GetDamageReceiver) Damage))

(fn ConstructionScript)

(fn OnChase
  (bind _asactor (Utilities|Casting|CastToActor (AI|Components|Blackboard|GetValueasObject (AI|GetBlackboard (AI|GetAIController self)) (Variables|Default|GetTargetPlayerKey))))
  (if (> (Transformation|GetDistanceTo _asactor) (Variables|/Script/AIModule.PawnSensingComponent|GetSightRadius (Variables|Default|GetPawnSensing)))
    (CallFunction|SetState "NewEnumerator0")))

(fn OnAttack
  (bind _asbp_character (Utilities|Casting|CastToBP_Character (AI|Components|Blackboard|GetValueasObject (AI|GetBlackboard (AI|GetAIController self)) (Variables|Default|GetTargetPlayerKey))))
  (if (Utilities|Enum|Equal(Enum) (Variables|/Game/Blueprint/Character/BP_Character.BP_Character_C|GetCharacterState _asbp_character) "NewEnumerator2")
    (CallFunction|SetState "NewEnumerator0")))