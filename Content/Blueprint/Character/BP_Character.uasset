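; Combat character that, outside StartMap, spawns a random sword, hammer or dagger on its hand socket and takes its attack speed.
; Damage goes to a DamageReceiver, whose health changes update HP percent on the possessing BP_PlayerController.
; Death disables capsule collision, zeroes walk speed and sets a final state that SetState never leaves.
; Attack check begin and end events forward to the equipped weapon.
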(event Custom|OnHpChanged
  (params (MaxHealthPower :type Float%20%28double-precision%29) (currentHealthPower :type Float%20%28double-precision%29))
  (Utilities|IsValid (Variables|Default|GetPlayerController)
    (:Is%20Valid
      (Default|SetHPPercent (Variables|Default|GetPlayerController) (/ currentHealthPower MaxHealthPower)))))

(event Custom|OnAttackCheckBegin
  (Default|OnAttackCheckBegin (Variables|Default|GetWeapon)))

(event Custom|OnAttackCheckEnd
  (Default|OnAttackCheckEnd (Variables|Default|GetWeapon)))

(event Custom|OnDead
  (Collision|SetCollisionEnabled (Variables|Collision|GetCapsuleComponent) "NoCollision")
  (CallFunction|SetState "NewEnumerator2")
  (Variables|/Script/Engine.CharacterMovementComponent|SetMaxWalkSpeed (Variables|Character|GetCharacterMovement) 0.0))

(event Custom|SetState
  (params (NewState :type ECharacterState%20Enum :default "NewEnumerator0"))
  (if (Utilities|Enum|NotEqual(Enum) NewState (Variables|Default|GetCharacterState))
    (if (Utilities|Enum|NotEqual(Enum) (Variables|Default|GetCharacterState) "NewEnumerator2")
      (Variables|Default|SetCharacterState NewState))))

(event EventBeginPlay
  (bind _returnvalue (Game|GetCurrentLevelName true))
  (if (Utilities|Enum|NotEqual(Enum) _returnvalue "StartMap")
    (bind _weapon (CallFunction|SpawnRandomWeapon))
    (Transformation|AttachComponentToComponent _weapon (Variables|Character|GetMesh) "WeaponPosition" "SnapToTarget" "SnapToTarget" "SnapToTarget" true)
    (bind _output_get (Variables|Default|SetWeapon _weapon))
    (Variables|Default|SetCurrentAttackSpeed (Variables|/Game/Blueprint/Character/Weapon/BP_Weapon.BP_Weapon_C|GetAttackSpeed _output_get))
    (Variables|Default|SetHasWeapon true)
    (EventDispatchers|BindEventtoOnHealthPowerChanged (Variables|Default|GetDamageReceiver) (delegate Custom|OnHpChanged))
    (EventDispatchers|BindEventtoOnDead (Variables|Default|GetDamageReceiver) (delegate Custom|OnDead))))

(event Game|Damage|EventAnyDamage
  (params (Damage :type Float%20%28single-precision%29) (DamageType :type Damage%20Type%20Object%20Reference) (InstigatedBy :type Controller%20Object%20Reference) (DamageCauser :type Actor%20Object%20Reference))
  (Default|OnDamageReceived (Variables|Default|GetDamageReceiver) Damage))

(event EventPossessed
  (params (NewController :type Controller%20Object%20Reference))
  (bind _asbp_player_controller (Utilities|Casting|CastToBP_PlayerController NewController))
  (Variables|Default|SetPlayerController _asbp_player_controller))

(fn ConstructionScript)

(fn SpawnRandomWeapon
  (switch int (Math|Integer|%(Integer) (Math|Random|RandomIntegerinRange 0 (Variables|Default|GetRanMax)) (Variables|Default|GetWeaponNum))
    (:0
      (bind _weapon (CallFunction|SpawnWeaponbyType "/Game/Blueprint/Character/Weapon/BP_Sword.BP_Sword_C"))
      (Variables|Default|SetWeaponClass "/Game/Blueprint/Character/Weapon/BP_Sword.BP_Sword_C")
      (return _weapon))
    (:1
      (bind _weapon_2 (CallFunction|SpawnWeaponbyType "/Game/Blueprint/Character/Weapon/BP_Hammer.BP_Hammer_C"))
      (Variables|Default|SetWeaponClass 0)
      (return _weapon_2))
    (:2
      (bind _weapon_3 (CallFunction|SpawnWeaponbyType "/Game/Blueprint/Character/Weapon/BP_Dagger.BP_Dagger_C"))
      (Variables|Default|SetWeaponClass 0)
      (return _weapon_3))))

(fn SpawnWeaponbyType
  (params (SpawnClass :type BP%20Weapon%20Class%20Reference))
  (bind _returnvalue (Game|SpawnActorfromClass SpawnClass (Math|Transform|MakeTransform "0, 0, 0") "Undefined" "MultiplyWithRoot" 0 0))
  (return _returnvalue))