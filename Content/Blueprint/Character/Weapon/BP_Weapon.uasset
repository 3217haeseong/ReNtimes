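; BP_Weapon is a weapon actor that deals damage to actors its attack collision overlaps.
; On BeginPlay it looks up its attack power and attack speed by WeaponName from WeaponData.
; Attack check begin and end events switch the collision between query-only and disabled to limit the hit window.
; Each overlap applies damage with player controller 0 as instigator and the weapon as causer.
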(event OnComponentBeginOverlap(AttackCollision)
  (params (OverlappedComponent :type Primitive%20Component%20Object%20Reference) (OtherActor :type Actor%20Object%20Reference) (OtherComp :type Primitive%20Component%20Object%20Reference) (OtherBodyIndex :type Integer) (bFromSweep :type Boolean) (SweepResult :type Hit%20Result%20Structure%20%28by%20ref%29))
  ;[0.15 0.15 0.15 0.5] 물체가 오버랩되면 ApplyDamage 호출
  (Game|Damage|ApplyDamage OtherActor (Variables|Default|GetBase%20Damage) (Game|GetPlayerController 0) self))

(event Custom|OnAttackCheckBegin
  ;[0.15 0.15 0.15 0.5] 공격 시작과 끝에 콜리전 관리
  (Collision|SetCollisionEnabled (Variables|Default|GetAttackCollision) "QueryOnly"))

(event Custom|OnAttackCheckEnd
  ;[0.15 0.15 0.15 0.5] 공격 시작과 끝에 콜리전 관리
  (Collision|SetCollisionEnabled (Variables|Default|GetAttackCollision) "NoCollision"))

(event EventBeginPlay
  (bind _weapondata (Variables|Default|GetWeaponData))
  (bind _weaponname (Variables|Default|GetWeaponName))
  (bind _weapondata_2 (Default|GetDatabyName _weapondata _weaponname))
  (Variables|Default|SetBase%20Damage (.attackpower _weapondata_2))
  (Variables|Default|SetAttackSpeed (.attackspeed _weapondata_2)))

(event Collision|EventActorBeginOverlap
  (params (OtherActor :type Actor%20Object%20Reference)))

(event EventTick
  (params (DeltaSeconds :type Float%20%28single-precision%29)))

(fn ConstructionScript)